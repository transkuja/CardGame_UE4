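; Blueprint function library of lookup helpers linking card effects, resources and their visuals in a card game.
; Two switch functions convert between the Red, Blue and Green resources and their resource-raising card effects, with non-resource effects mapping to None.
; Two more pick an icon sprite and color per effect.
; Resource effects share one ball sprite, told apart by color, while Draw reuses green and Damage red.
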(fn GetResourcefromCardEffect
  (params (CardEffect :type CardEffect%20Enum :default "NewEnumerator3"))
  (switch Utilities|FlowControl|Switch|SwitchonCardEffect CardEffect
    (:NewEnumerator3
      _)
    (:NewEnumerator0
      _)
    (:NewEnumerator1
      _)
    (:NewEnumerator2
      (return "NewEnumerator0"))
    (:NewEnumerator4
      (return "NewEnumerator1"))
    (:NewEnumerator5
      (return "NewEnumerator2")))
  (return "NewEnumerator4"))

(fn GetCardEffectfromResource
  (params (Resource :type Resources%20Enum :default "NewEnumerator4"))
  (switch Utilities|FlowControl|Switch|SwitchonResources Resource
    (:NewEnumerator4
      (return "NewEnumerator3"))
    (:NewEnumerator0
      (return "NewEnumerator2"))
    (:NewEnumerator1
      (return "NewEnumerator4"))
    (:NewEnumerator2
      (return "NewEnumerator5"))))

(fn GetSpritefromCardEffect
  (params (Card%20Effect :type CardEffect%20Enum :default "NewEnumerator3"))
  (switch Utilities|FlowControl|Switch|SwitchonCardEffect Card%20Effect
    (:NewEnumerator0
      (return "/Game/Sprites/card-draw256_Sprite.card-draw256_Sprite"))
    (:NewEnumerator1
      (return "/Game/Sprites/crossed-swords256_Sprite.crossed-swords256_Sprite"))
    (:NewEnumerator2
      _)
    (:NewEnumerator4
      _)
    (:NewEnumerator5
      _))
  (return "/Game/Sprites/glass-ball-small_Sprite.glass-ball-small_Sprite"))

(fn GetColorfromCardEffect
  (params (Card%20Effect :type CardEffect%20Enum :default "NewEnumerator3"))
  (switch Utilities|FlowControl|Switch|SwitchonCardEffect Card%20Effect
    (:NewEnumerator0
      _)
    (:NewEnumerator1
      (return (Math|Color|MakeColor 0 0 237 255)))
    (:NewEnumerator2
      (return (Math|Color|MakeColor 0 0 237 255)))
    (:NewEnumerator4
      (return (Math|Color|MakeColor 255 127 0 255)))
    (:NewEnumerator5
      _))
  (return (Math|Color|MakeColor 88 215 1 255)))