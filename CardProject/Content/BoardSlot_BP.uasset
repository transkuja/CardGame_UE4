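; Board slot actor where the player places a card, which then applies its "on set" effects each time a turn begins.
; Clicking its plane takes the player's selected card if card plays remain this turn and its costs can be met.
; Placement sends the previous card to discard, moves the new one out of the hand onto the slot, pays costs and notifies the TurnHandler.
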(event OnClicked(Plane)
  (params (TouchedComponent :type Primitive%20Component%20Object%20Reference) (ButtonPressed :type Key%20Structure))
  (CallFunction|AddCardtoBoard))

(event Custom|OnBeginTurn
  (CallFunction|ApplySetCardEffect))

(event EventBeginPlay
  (EventDispatchers|AssignOnBeginTurnED (Variables|/Game/Player/CustomPlayerCharacter.CustomPlayerCharacter_C|GetTurn%20Handler (.AsCustom%20Player%20Character (Utilities|Casting|CastToCustomPlayerCharacter (Game|GetPlayerCharacter 0)))) (delegate Custom|OnBeginTurn)))

(event Collision|EventActorBeginOverlap
  (params (OtherActor :type Actor%20Object%20Reference)))

(event EventTick
  (params (DeltaSeconds :type Float%20%28single-precision%29)))

(fn ConstructionScript)

(fn AddCardtoBoard
  (bind _returnvalue (Game|GetPlayerCharacter 0))
  (bind _returnvalue_2 (Game|GetPlayerCharacter 0))
  (bind _returnvalue_3 (Game|GetPlayerCharacter 0))
  (bind _ascustom_player_character (Utilities|Casting|CastToCustomPlayerCharacter _returnvalue))
  (bind _ascustom_player_character_2 (Utilities|Casting|CastToCustomPlayerCharacter _returnvalue_3))
  (bind _ascustom_player_character_3 (Utilities|Casting|CastToCustomPlayerCharacter _returnvalue_2))
  (if (> (Variables|/Game/TurnHandler_BP.TurnHandler_BP_C|GetCurrentTurnCardsLeft (Variables|/Game/Player/CustomPlayerCharacter.CustomPlayerCharacter_C|GetTurn%20Handler _ascustom_player_character_2)) 0)
    (Utilities|IsValid (Variables|/Game/Player/CustomPlayerCharacter.CustomPlayerCharacter_C|GetCurrently%20Clicked%20Card _ascustom_player_character_2)
      (:Is%20Valid
        (bind _canpaythecost (Default|CheckCosts (Variables|/Game/Card/Card_BP.Card_BP_C|GetCardData_BP (Variables|/Game/Player/CustomPlayerCharacter.CustomPlayerCharacter_C|GetCurrently%20Clicked%20Card _ascustom_player_character_2))))
        (if _canpaythecost
          (if (!= (Variables|/Game/Player/CustomPlayerCharacter.CustomPlayerCharacter_C|GetCurrently%20Clicked%20Card _ascustom_player_character_2) (Variables|Default|GetCard%20Ref))
            (Default|ToDiscardPile _ascustom_player_character (Variables|Default|GetCard%20Ref))
            (bind _output_get (Variables|Default|SetCard%20Ref (Variables|/Game/Player/CustomPlayerCharacter.CustomPlayerCharacter_C|GetCurrently%20Clicked%20Card _ascustom_player_character_2)))
            (Transformation|SetActorLocationAndRotation _output_get (- (Transformation|GetActorLocation) "-10.000000, 0,200.000000"))
            (Variables|/Game/Card/Card_BP.Card_BP_C|SetLocationOnBoard (Variables|/Game/Player/CustomPlayerCharacter.CustomPlayerCharacter_C|GetCurrently%20Clicked%20Card _ascustom_player_character_2) "NewEnumerator3")
            (Utilities|Array|RemoveItem (Variables|/Game/Player/CustomPlayerCharacter.CustomPlayerCharacter_C|GetCardsInHand _ascustom_player_character) _output_get)
            (Variables|/Game/Player/CustomPlayerCharacter.CustomPlayerCharacter_C|SetCurrently%20Clicked%20Card _ascustom_player_character_3 0)
            (Variables|/Game/Card/Card_BP.Card_BP_C|SetBoard%20Slot (Variables|Default|GetCard%20Ref) self)
            (Default|AdaptCardsinHandRotation _ascustom_player_character_3)
            (Default|PayCosts (Variables|/Game/Card/Card_BP.Card_BP_C|GetCardData_BP (Variables|Default|GetCard%20Ref)))
            (Default|CallOnCardUseED (Variables|/Game/Player/CustomPlayerCharacter.CustomPlayerCharacter_C|GetTurn%20Handler (.AsCustom%20Player%20Character (Utilities|Casting|CastToCustomPlayerCharacter (Game|GetPlayerCharacter 0))))))))
      (:Is%20Not%20Valid
        (Development|PrintString "Empty")))))

(fn ApplySetCardEffect
  (bind _card_ref (Variables|Default|GetCard%20Ref))
  (bind _carddata_bp (Variables|/Game/Card/Card_BP.Card_BP_C|GetCardData_BP _card_ref))
  (if (Utilities|IsValid (Variables|Default|GetCard%20Ref))
    (Default|CardUseSwitch _carddata_bp (.cardeffectsonset (Variables|/Game/Card/CardData_BP.CardData_BP_C|GetCardData _carddata_bp)))))