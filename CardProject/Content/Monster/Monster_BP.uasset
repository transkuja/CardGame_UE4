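; Monster actor that loads its stats, name and sprite from the MonsterDatabase data table by ID.
; CurrentHp starts at zero and ReceiveDamage adds to it, so the HP widget's progress bar fills up as damage lands.
; When CurrentHp exactly equals MaxHp, the sprite switches to the happy visual and a "Win!" debug message prints.
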(event EventBeginPlay)

(event Collision|EventActorBeginOverlap
  (params (OtherActor :type Actor%20Object%20Reference)))

(event EventTick
  (params (DeltaSeconds :type Float%20%28single-precision%29)))

(fn ConstructionScript)

(fn LoadMonsterData
  (params (MonsterId :type String))
  (bind _returnvalue (Utilities|GetDataTableRow "/Game/Monster/MonsterDatabase.MonsterDatabase" (Utilities|String|StringToName MonsterId))
    (:then
      (bind _output_get (Variables|Default|SetMonsterData _returnvalue))
      (Variables|Default|SetCurrentHp 0)
      (CallFunction|UpdateProgressBar)
      (Rendering|Components|Sprite|SetSprite (Variables|Default|GetVisual) (.visual _output_get))
      (Rendering|Components|TextRender|SetText (Variables|Default|GetName) (Utilities|Text|ToText(String) (.name _output_get))))))

(fn UpdateProgressBar
  (bind _monsterdata (Variables|Default|GetMonsterData))
  (bind _currenthp (Variables|Default|GetCurrentHp))
  (bind _maxhp (Utilities|Struct|BreakMonsterData _monsterdata))
  (Progress|SetPercent (Variables|/Game/Monster/MonsterProgressBar_BP.MonsterProgressBar_BP_C|GetProgressBar_41 (.AsMonster%20Progress%20Bar%20BP (Utilities|Casting|CastToMonsterProgressBar_BP (UserInterface|GetUserWidgetObject (Variables|Default|GetHP))))) (/ (Math|Conversions|ToFloat(Integer) _currenthp) (Math|Conversions|ToFloat(Integer) _maxhp)))
  (if (== _currenthp _maxhp)
    (Rendering|Components|Sprite|SetSprite (Variables|Default|GetVisual) (.happyvisual (Variables|Default|GetMonsterData)))
    (Development|PrintString "Win!" true true "(R=1.000000,G=0.109375,B=0.748525,A=1.000000)" 1e+01)))

(fn ReceiveDamage
  (params (Damage :type Integer))
  (Variables|Default|SetCurrentHp (+ (Variables|Default|GetCurrentHp) Damage))
  (CallFunction|UpdateProgressBar))