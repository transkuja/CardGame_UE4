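; Card data component on a Card_BP that loads a card's row from the card data table and handles playing it.
; UseCard checks the player's resources against costs, applies effects, discards the card, pays costs, then notifies the TurnHandler.
; Effects come from an enum-keyed map switched to draw cards, damage the board's spawned monster, or raise red, blue or green resources.
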(event Custom|UseCard
  (bind _canpaythecost (CallFunction|CheckCosts))
  (if _canpaythecost
    (CallFunction|CardUseSwitch (.cardeffectsonuse (Variables|Default|GetCardData)))
    (Default|ToDiscardPile (.AsCustom%20Player%20Character (Utilities|Casting|CastToCustomPlayerCharacter (Game|GetPlayerCharacter 0))) (.AsCard%20BP (Utilities|Casting|CastToCard_BP (Components|GetOwner))))
    (CallFunction|PayCosts)
    (Default|CallOnCardUseED (Variables|/Game/Player/CustomPlayerCharacter.CustomPlayerCharacter_C|GetTurn%20Handler (.AsCustom%20Player%20Character (Utilities|Casting|CastToCustomPlayerCharacter (Game|GetPlayerCharacter 0)))))))

(event EventBeginPlay)

(event EventTick
  (params (DeltaSeconds :type Float%20%28single-precision%29)))

(fn LoadCardData
  (params (Card%20Id :type Integer))
  (bind _outrownames (DataTable|GetDataTableRowNames "/Game/Card/CardDatabase.CardDatabase"))
  (bind _returnvalue (Utilities|GetDataTableRow "/Game/Card/CardDatabase.CardDatabase" (Utilities|Array|Get(acopy) _outrownames Card%20Id))
    (:then
      (bind _output_get (Variables|Default|SetCardData _returnvalue))
      (return (.name _output_get) (.description _output_get) (.value1 _output_get) (.value2 _output_get) (.visual _output_get)))))

(fn CardUseSwitch
  (params (Effects :type Map%20of%20CardEffect%20Enums%20to%20Integers :default "NewEnumerator3"))
  (bind _returnvalue (Game|GetPlayerCharacter 0))
  (bind _ascustom_player_character (Utilities|Casting|CastToCustomPlayerCharacter _returnvalue))
  (bind _resources (Variables|/Game/Player/CustomPlayerCharacter.CustomPlayerCharacter_C|GetResources _ascustom_player_character))
  (bind _keys (Utilities|Map|Keys Effects))
  (for (_array_element _array_index) _keys
    (bind _values (Utilities|Map|Values Effects))
    (switch Utilities|FlowControl|Switch|SwitchonCardEffect _array_element
      (:NewEnumerator0
        ;[1 1 1] Draw x cards
        (Default|DrawX (.AsCustom%20Player%20Character (Utilities|Casting|CastToCustomPlayerCharacter (Game|GetPlayerCharacter 0))) (Utilities|Array|Get(acopy) _values _array_index)))
      (:NewEnumerator1
        ;[1 1 1] Deal X damage
        (Default|ReceiveDamage (Variables|/Game/Board_BP.Board_BP_C|GetSpawned%20Monster (Variables|/Game/Player/CustomPlayerCharacter.CustomPlayerCharacter_C|GetBoard%20Reference _ascustom_player_character)) (Utilities|Array|Get(acopy) _values _array_index)))
      (:NewEnumerator2
        ;[1 1 1] Update resources
        (bind _resource (CallFunction|GetResourcefromCardEffect _array_element :!label _label))
        (bind _output_get (LocalVariables|SetTmpAddToMap (+ (.Value (Utilities|Map|Find _resources _resource)) (Utilities|Array|Get(acopy) _values _array_index))))
        (Utilities|Map|Remove _resources _resource)
        (Utilities|Map|Add _resources _resource _output_get))
      (:NewEnumerator4
        (goto _label))
      (:NewEnumerator5
        (goto _label)))))

(fn CheckCosts
  (bind _carddata (Variables|Default|GetCardData))
  (bind _keys (Utilities|Map|Keys (.costs _carddata)))
  (for _array_element _keys
    (if (not (<= (.Value (Utilities|Map|Find (.costs _carddata) _array_element)) (.Value (Utilities|Map|Find (Variables|/Game/Player/CustomPlayerCharacter.CustomPlayerCharacter_C|GetResources (.AsCustom%20Player%20Character (Utilities|Casting|CastToCustomPlayerCharacter (Game|GetPlayerCharacter 0)))) _array_element))))
      (return (<= (.Value (Utilities|Map|Find (.costs _carddata) _array_element)) (.Value (Utilities|Map|Find (Variables|/Game/Player/CustomPlayerCharacter.CustomPlayerCharacter_C|GetResources (.AsCustom%20Player%20Character (Utilities|Casting|CastToCustomPlayerCharacter (Game|GetPlayerCharacter 0)))) _array_element))))))
  (return true))

(fn PayCosts
  (bind _returnvalue (Game|GetPlayerCharacter 0))
  (bind _carddata (Variables|Default|GetCardData))
  (bind _ascustom_player_character (Utilities|Casting|CastToCustomPlayerCharacter _returnvalue))
  (bind _resources (Variables|/Game/Player/CustomPlayerCharacter.CustomPlayerCharacter_C|GetResources _ascustom_player_character))
  (bind _keys (Utilities|Map|Keys (.costs _carddata)))
  (for _array_element _keys
    (bind _output_get (LocalVariables|SetTmpAddToMap (- (.Value (Utilities|Map|Find _resources _array_element)) (.Value (Utilities|Map|Find (.costs _carddata) _array_element)))))
    (Utilities|Map|Remove _resources _array_element)
    (Utilities|Map|Add _resources _array_element _output_get)
    (Development|PrintString (Utilities|String|EnumtoString _array_element))))