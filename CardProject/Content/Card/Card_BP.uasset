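; Card actor for a card game that reacts to mouse hover and clicks according to its location: hand, deck, discard or board.
; Hovering a hand card raises it and brings it forward using offsets from CustomPlayerCharacter; clicking toggles that player's currently clicked card.
; Deck clicks draw, discard clicks draw only when the deck is empty, and board clicks call the overlapped BoardSlot_BP.
; InitData loads card data by index through CardDataBP.
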(event OnClicked(Background)
  (params (TouchedComponent :type Primitive%20Component%20Object%20Reference) (ButtonPressed :type Key%20Structure))
  ;[1 1 1] Draw from deck
  (Default|Draw (.AsCustom%20Player%20Character (Utilities|Casting|CastToCustomPlayerCharacter (Game|GetPlayerCharacter 0)))))

(event OnComponentBeginOverlap(Support)
  (params (OverlappedComponent :type Primitive%20Component%20Object%20Reference) (OtherActor :type Actor%20Object%20Reference) (OtherComp :type Primitive%20Component%20Object%20Reference) (OtherBodyIndex :type Integer) (bFromSweep :type Boolean) (SweepResult :type Hit%20Result%20Structure%20%28by%20ref%29))
  (bind _asboard_slot_bp (Utilities|Casting|CastToBoardSlot_BP OtherActor))
  (Variables|Default|SetBoard%20Slot _asboard_slot_bp)
  (Development|PrintString "Board slot set" true true "(R=0.000000,G=0.660000,B=1.000000,A=1.000000)" 1e+01))

(event OnComponentEndOverlap(Support)
  (params (OverlappedComponent :type Primitive%20Component%20Object%20Reference) (OtherActor :type Actor%20Object%20Reference) (OtherComp :type Primitive%20Component%20Object%20Reference) (OtherBodyIndex :type Integer))
  (Utilities|Casting|CastToBoardSlot_BP OtherActor)
  (Variables|Default|SetBoard%20Slot 0)
  (Development|PrintString "Board slot freed" true true "(R=0.000000,G=0.660000,B=1.000000,A=1.000000)" 1e+01))

(event OnBeginCursorOver(Support)
  (params (TouchedComponent :type Primitive%20Component%20Object%20Reference))
  (CallFunction|ShowCard))

(event OnEndCursorOver(Support)
  (params (TouchedComponent :type Primitive%20Component%20Object%20Reference))
  (CallFunction|HideCard))

(event OnClicked(Support)
  (params (TouchedComponent :type Primitive%20Component%20Object%20Reference) (ButtonPressed :type Key%20Structure))
  (bind _returnvalue (Game|GetPlayerCharacter 0))
  (bind _returnvalue_2 (Game|GetPlayerCharacter 0))
  (bind _ascustom_player_character (Utilities|Casting|CastToCustomPlayerCharacter _returnvalue_2))
  (bind _ascustom_player_character_2 (Utilities|Casting|CastToCustomPlayerCharacter _returnvalue))
  (switch Utilities|FlowControl|Switch|SwitchonCardPosition (Variables|Default|GetLocationOnBoard)
    (:NewEnumerator0
      (Utilities|IsValid (Variables|/Game/Player/CustomPlayerCharacter.CustomPlayerCharacter_C|GetCurrently%20Clicked%20Card _ascustom_player_character)
        (:Is%20Valid
          (Variables|/Game/Player/CustomPlayerCharacter.CustomPlayerCharacter_C|SetCurrently%20Clicked%20Card _ascustom_player_character 0)
          (Development|PrintString "free"))
        (:Is%20Not%20Valid
          (Variables|/Game/Player/CustomPlayerCharacter.CustomPlayerCharacter_C|SetCurrently%20Clicked%20Card _ascustom_player_character self)
          (Development|PrintString "Hello"))))
    (:NewEnumerator1
      (Default|Draw _ascustom_player_character)
      (Variables|/Game/Player/CustomPlayerCharacter.CustomPlayerCharacter_C|SetCurrently%20Clicked%20Card _ascustom_player_character_2 0))
    (:NewEnumerator2
      ;[1 1 1] If has clicked on face up card and there's no card left in deck, shuffle discard into deck then draw
      (Variables|/Game/Player/CustomPlayerCharacter.CustomPlayerCharacter_C|SetCurrently%20Clicked%20Card _ascustom_player_character_2 0)
      (if (== (Utilities|Array|Length (Variables|/Game/Player/CustomPlayerCharacter.CustomPlayerCharacter_C|GetDeck _ascustom_player_character)) 0)
        (Default|Draw (.AsCustom%20Player%20Character (Utilities|Casting|CastToCustomPlayerCharacter (Game|GetPlayerCharacter 0))))))
    (:NewEnumerator3
      (Default|AddCardtoBoard (Variables|Default|GetBoard%20Slot)))))

(event Custom|OnMouseReleased)

(event EventBeginPlay)

(event Collision|EventActorBeginOverlap
  (params (OtherActor :type Actor%20Object%20Reference)))

(event EventTick
  (params (DeltaSeconds :type Float%20%28single-precision%29)))

(fn ConstructionScript)

(fn InitData
  (params (CardIndex :type Integer))
  (Default|LoadCardData (Variables|Default|GetCardData_BP) CardIndex))

(fn ShowCard
  (if (Utilities|Enum|Equal(Enum) (Variables|Default|GetLocationOnBoard) "NewEnumerator0")
    (bind _output_get (Variables|Default|SetDefaultPosition (Transformation|GetActorLocation)))
    (bind _x_ahead (Default|PutCardinHandAhead (.AsCustom%20Player%20Character (Utilities|Casting|CastToCustomPlayerCharacter (Game|GetPlayerCharacter 0)))))
    (Transformation|SetActorLocation (Math|Vector|MakeVector _x_ahead (.y (+ _output_get (* (Transformation|GetActorUpVector) (LocalVariables|GetMoveStep)))) (.z (+ _output_get (* (Transformation|GetActorUpVector) (LocalVariables|GetMoveStep))))) false false)))

(fn HideCard
  (bind _defaultposition (Variables|Default|GetDefaultPosition))
  (if (Utilities|Enum|Equal(Enum) (Variables|Default|GetLocationOnBoard) "NewEnumerator0")
    (bind _x_offset (Default|GetXOffsetfromPositioninHand (.AsCustom%20Player%20Character (Utilities|Casting|CastToCustomPlayerCharacter (Game|GetPlayerCharacter 0))) self))
    (Transformation|SetActorLocation (Math|Vector|MakeVector _x_offset (.y _defaultposition) (.z _defaultposition)) false false)))