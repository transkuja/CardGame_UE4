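; Board actor that hosts three card slots and a monster, placed at its own location components.
; On BeginPlay it spawns a BoardSlot_BP at each of the three card locations and stores them in Slots.
; SpawnMonster looks up the ID in MonsterDatabase and, only if the row exists, spawns a Monster_BP at MonsterLocation.
; The monster is kept as SpawnedMonster and receives the ID, not the row, to load its own data.
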(event EventBeginPlay
  (bind _returnvalue (Game|SpawnActorfromClass "/Game/BoardSlot_BP.BoardSlot_BP_C" (Transformation|GetWorldTransform (Variables|Default|GetCard1Location)) "Undefined" 0 0))
  (Utilities|Array|Add (Variables|Default|GetSlots) _returnvalue)
  (bind _returnvalue_2 (Game|SpawnActorfromClass "/Game/BoardSlot_BP.BoardSlot_BP_C" (Transformation|GetWorldTransform (Variables|Default|GetCard2Location)) "Undefined" 0 0))
  (Utilities|Array|Add (Variables|Default|GetSlots) _returnvalue_2)
  (bind _returnvalue_3 (Game|SpawnActorfromClass "/Game/BoardSlot_BP.BoardSlot_BP_C" (Transformation|GetWorldTransform (Variables|Default|GetCard3Location)) "Undefined" 0 0))
  (Utilities|Array|Add (Variables|Default|GetSlots) _returnvalue_3))

(event Collision|EventActorBeginOverlap
  (params (OtherActor :type Actor%20Object%20Reference)))

(event EventTick
  (params (DeltaSeconds :type Float%20%28single-precision%29)))

(fn ConstructionScript)

(fn SpawnMonster
  (params (Monster%20id :type String))
  (Utilities|GetDataTableRow "/Game/Monster/MonsterDatabase.MonsterDatabase" (Utilities|String|StringToName Monster%20id)
    (:then
      (bind _returnvalue (Game|SpawnActorfromClass "/Game/Monster/Monster_BP.Monster_BP_C" (Transformation|GetWorldTransform (Variables|Default|GetMonster%20Location)) "Undefined" 0 0))
      (bind _output_get (Variables|Default|SetSpawned%20Monster _returnvalue))
      (Default|LoadMonsterData _output_get Monster%20id))))