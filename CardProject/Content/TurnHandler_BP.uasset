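; TurnHandler_BP manages the turn cycle of a card game, tracking how many cards remain playable in the current turn.
; Each turn start resets that count to the per-turn maximum and broadcasts a begin-turn event dispatcher.
; Bound dispatchers decrement the count on card use and start the next turn on turn end.
; A comment notes that monsters should act before the next turn begins, but no such step exists here.
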(event Custom|OnEndTurn
  ;[0.7344 0 0.02521] Monsters should play their turns before calling OnBeginTurn
  (CallFunction|OnBeginTurn))

(event Custom|OnCardUse
  (Math|Integer|DecrementInt (Variables|Default|GetCurrentTurnCardsLeft)))

(event EventBeginPlay
  (CallFunction|OnBeginTurn)
  (EventDispatchers|BindEventtoOnCardUseED (delegate Custom|OnCardUse))
  ;[0.7344 0 0.02521] Monsters should play their turns before calling OnBeginTurn
  (EventDispatchers|BindEventtoOnEndTurnED (delegate Custom|OnEndTurn)))

(event Collision|EventActorBeginOverlap
  (params (OtherActor :type Actor%20Object%20Reference)))

(event EventTick
  (params (DeltaSeconds :type Float%20%28single-precision%29)))

(fn ConstructionScript)

(fn OnBeginTurn
  (Variables|Default|SetCurrentTurnCardsLeft (Variables|Default|GetMaxCardPerTurn))
  (Default|CallOnBeginTurnED))